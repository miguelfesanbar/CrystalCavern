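; Player pawn that moves by applying physics torque to its mesh.
; The forward/backward and right/left input axes add torque around Y and X respectively, scaled by a strength variable and applied as acceleration change, so mass is ignored.
; On BeginPlay it runs a camera fade from full opacity to bring the view in.
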(event `self.ReceiveBeginPlay`
  (`PlayerCameraManager.StartCameraFade` :`self` (`GameplayStatics.GetPlayerCameraManager` 0) :`FromAlpha` 1.0 :`Duration` 2.0 :`bHoldWhenFinished` true))

(event `InputAxis|Move Forward/Backwards`
  (params (AxisValue :type "Float (single-precision)"))
  (`PrimitiveComponent.AddTorqueInRadians` (`self.Mesh`) (`KismetMathLibrary.MakeVector` 0.0 (* AxisValue (`self.strenght`))) "None" true))

(event `InputAxis|Move Right/Left`
  (params (AxisValue :type "Float (single-precision)"))
  (`PrimitiveComponent.AddTorqueInRadians` (`self.Mesh`) (`KismetMathLibrary.MakeVector` (* AxisValue (`self.strenght`))) "None" true))

(fn `UserConstructionScript`)